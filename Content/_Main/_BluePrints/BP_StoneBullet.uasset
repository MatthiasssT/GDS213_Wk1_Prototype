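; BP_StoneBullet is a stone projectile that damages actors tagged "Enemy" on impact, crediting the player character as damage causer.
; On BeginPlay its Cone component is set to ignore the player while moving.
; A ProjectileMovement bounce off an enemy applies point damage, turns on Cone physics simulation, then destroys the bullet after a short delay with a debug print.
; Bounces off other actors trigger no logic.
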(event OnProjectileBounce(ProjectileMovement)
  (params (ImpactResult :type Hit%20Result%20Structure%20%28by%20ref%29) (ImpactVelocity :type Vector%20%28by%20ref%29 :default "0, 0, 0"))
  (bind _hitactor (Collision|BreakHitResult ImpactResult))
  (if (Actor|ActorHasTag _hitactor "Enemy")
    (Game|Damage|ApplyPointDamage _hitactor (Variables|Default|GetDamageDealt) ImpactVelocity ImpactResult 0 (Variables|Default|GetPlayerC%20Ref) "/Script/Engine.DamageType")
    (Physics|SetSimulatePhysics (Variables|Default|GetCone) true)
    (Utilities|FlowControl|Delay 3.0)
    (Development|PrintString "bullet destroyed")
    (Actor|DestroyActor)))

(event EventBeginPlay
  (bind _output_get (Variables|Default|SetPlayerC%20Ref (Game|GetPlayerCharacter 0)))
  (Collision|IgnoreActorwhenMoving (Variables|Default|GetCone) _output_get true))

(event Collision|EventActorBeginOverlap
  (params (OtherActor :type Actor%20Object%20Reference)))

(event EventTick
  (params (DeltaSeconds :type Float%20%28single-precision%29)))

(fn ConstructionScript)
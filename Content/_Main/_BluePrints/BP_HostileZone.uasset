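; BP_HostileZone is a trigger zone that makes the player and enemies hostile while the player is inside it.
; It caches the BP_Player pawn on BeginPlay and filters Trigger overlaps by the "Player" tag.
; Entering switches the player and every BP_Enemy in the level to hostile, and leaving reverts them to neutral.
; Enemies are gathered with GetAllActorsOfClass on each overlap, so the effect is level-wide rather than local to the zone.
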(event OnComponentBeginOverlap(Trigger)
  (params (OverlappedComponent :type Primitive%20Component%20Object%20Reference) (OtherActor :type Actor%20Object%20Reference) (OtherComp :type Primitive%20Component%20Object%20Reference) (OtherBodyIndex :type Integer) (bFromSweep :type Boolean) (SweepResult :type Hit%20Result%20Structure%20%28by%20ref%29))
  (if (Actor|ActorHasTag OtherActor "Player")
    (Default|ChangeStatetoHostile (Variables|Default|GetAs%20BP%20Player))
    (bind _outactors (Actor|GetAllActorsOfClass "/Game/_Main/_BluePrints/BP_Enemy.BP_Enemy_C"))
    (for _array_element _outactors
      (Default|SetEnemyHostile _array_element))))

(event OnComponentEndOverlap(Trigger)
  (params (OverlappedComponent :type Primitive%20Component%20Object%20Reference) (OtherActor :type Actor%20Object%20Reference) (OtherComp :type Primitive%20Component%20Object%20Reference) (OtherBodyIndex :type Integer))
  (if (Actor|ActorHasTag OtherActor "Player")
    (Default|ChangeStatetoNeutral (Variables|Default|GetAs%20BP%20Player))
    (bind _outactors (Actor|GetAllActorsOfClass "/Game/_Main/_BluePrints/BP_Enemy.BP_Enemy_C"))
    (for _array_element _outactors
      (Default|SetEnemyNeutral _array_element))))

(event EventBeginPlay
  (bind _asbp_player (Utilities|Casting|CastToBP_Player (Game|GetPlayerCharacter 0)))
  (Variables|Default|SetAs%20BP%20Player _asbp_player))

(event Collision|EventActorBeginOverlap
  (params (OtherActor :type Actor%20Object%20Reference)))

(event EventTick
  (params (DeltaSeconds :type Float%20%28single-precision%29)))

(fn ConstructionScript)
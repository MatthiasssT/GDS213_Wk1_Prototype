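; BP_Enemy is an enemy with a health pool that starts at its maximum and drops when it is hit.
; It takes only point damage whose causer carries the Player tag, ignoring hits once dead, and prints the remaining health.
; When health falls below zero it flags itself dead, briefly waits, turns on mesh physics, then destroys itself after another short delay.
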(event Custom|LoseHealth
  (params (DamageTaken :type Float%20%28double-precision%29))
  (bind _output_get (Variables|Default|SetCurrentHealth (- (Variables|Default|GetCurrentHealth) DamageTaken)))
  (if (< _output_get 0.0)
    (CallFunction|Death)
    (else
      (Development|PrintString (Utilities|String|ToString(Float) _output_get)))))

(event Custom|Death
  (Variables|Default|SetIsDead? true)
  (Utilities|FlowControl|Delay 0.2)
  (Physics|SetSimulatePhysics (Variables|Character|GetMesh) true)
  (Utilities|FlowControl|Delay 0.5)
  (Actor|DestroyActor))

(event EventBeginPlay
  (Variables|Default|SetCurrentHealth (Variables|Default|GetMaxHealth)))

(event Collision|EventActorBeginOverlap
  (params (OtherActor :type Actor%20Object%20Reference)))

(event Game|Damage|EventPointDamage
  (params (Damage :type Float%20%28single-precision%29) (DamageType :type Damage%20Type%20Object%20Reference) (HitLocation :type Vector :default "0, 0, 0") (HitNormal :type Vector :default "0, 0, 0") (HitComponent :type Primitive%20Component%20Object%20Reference) (BoneName :type Name :default "None") (ShotFromDirection :type Vector :default "0, 0, 0") (InstigatedBy :type Controller%20Object%20Reference) (DamageCauser :type Actor%20Object%20Reference) (HitInfo :type Hit%20Result%20Structure%20%28by%20ref%29))
  (if (and (Actor|ActorHasTag DamageCauser "Player") (not (Variables|Default|GetIsDead?)))
    (CallFunction|LoseHealth Damage)))

(event EventTick
  (params (DeltaSeconds :type Float%20%28single-precision%29)))

(fn ConstructionScript)